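; Projectile actor that deals damage through its Box overlap, with separate branches labelled for enemy and player character.
; With a valid TargetDMG it damages only that actor; otherwise it damages the overlapped actor, without passing a damage type.
; Each branch fires once, reports an AI damage-sense event and destroys the projectile.
; The fallback report still passes the invalid TargetDMG as the damaged actor and omits the damage amount.
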(event `self.Box.OnComponentBeginOverlap`
  (params (OverlappedComponent :type "PrimitiveComponent Object Reference") (OtherActor :type "Actor Object Reference") (OtherComp :type "PrimitiveComponent Object Reference") (OtherBodyIndex :type Integer) (bFromSweep :type Boolean) (SweepResult :type "HitResult Structure (by ref)"))
  (bind _targetdmg (`self.TargetDMG`))
  (`self.TargetDMG`
    (:`then`
      ;[1 1 1] enemy
      (if (== OtherActor _targetdmg)
        (`/Engine/EditorBlueprintResources/StandardMacros.IsValid` _targetdmg
          (:`Is Valid`
            (`/Engine/EditorBlueprintResources/StandardMacros.DoOnce` false
              (:`Completed`
                (bind _returnvalue (`GameplayStatics.ApplyDamage` (`self.TargetDMG`) (`self.Base Damage`) null (`self.Damage Causer`) "/Script/Engine.DamageType"))
                (`AISense_Damage.ReportDamageEvent` (`self.TargetDMG`) (`self.Damage Causer`) _returnvalue (`self.K2_GetActorLocation`))
                (`self.K2_DestroyActor`)))))))
    (:`else`
      ;[1 1 1] player character
      (`/Engine/EditorBlueprintResources/StandardMacros.DoOnce` false
        (:`Completed`
          (`GameplayStatics.ApplyDamage` OtherActor (`self.Base Damage`) null (`self.Damage Causer`))
          (`AISense_Damage.ReportDamageEvent` (`self.TargetDMG`) (`self.Damage Causer`) 0.0 (`self.K2_GetActorLocation`))
          (`self.K2_DestroyActor`))))))

(event `self.ReceiveDestroyed`)

(fn `UserConstructionScript`)