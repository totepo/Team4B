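; Blueprint helper library for enemy AI that provides component lookups and combat damage math.
; Validity-checked getters return an actor's AI enemy, character movement, skeletal mesh or capsule component.
; CalculateDamage rolls a percentage against critical rate and adds the critical bonus percentage to attack on success.
; CalculateDefence reduces damage by the defence percentage, substituting a minimal value only when the result is exactly zero.
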(fn GetAIEnemyComp
  (params (Actor :type Actor%20Object%20Reference))
  (Utilities|IsValid Actor
    (:Is%20Valid
      (return (Actor|GetComponentbyClass Actor "/Game/AIEnemy_/C_AIEnemyComponet.C_AIEnemyComponet_C")))))

(fn GetMovtComp
  (params (Target :type Actor%20Object%20Reference))
  (Utilities|IsValid Target
    (:Is%20Valid
      (return (Actor|GetComponentbyClass Target "/Script/Engine.CharacterMovementComponent")))))

(fn GetSkeletalComp
  (params (actor :type Actor%20Object%20Reference))
  (Utilities|IsValid actor
    (:Is%20Valid
      (return (Actor|GetComponentbyClass actor "/Script/Engine.SkeletalMeshComponent")))))

(fn GetCapsuleComp
  (params (Actor :type Actor%20Object%20Reference))
  (Utilities|IsValid Actor
    (:Is%20Valid
      (return (Actor|GetComponentbyClass Actor "/Script/Engine.CapsuleComponent")))))

(fn CalculateDamage
  (params (Attack :type Float%20%28double-precision%29) (CriticalR :type Float%20%28double-precision%29) (CriticalP :type Float%20%28double-precision%29))
  (LocalVariables|SetCPActor CriticalP)
  (LocalVariables|SetCRActor CriticalR)
  (LocalVariables|SetDañoActor Attack)
  (Math|Integer|CompareInt (Math|Random|RandomIntegerinRange 1 100) (Math|Float|Round (LocalVariables|GetCRActor))
    (:>
      (return (LocalVariables|GetDañoActor)))
    (:==
      _)
    (:<
      _))
  (return (|(Dmg+(Dmg*CP)) (LocalVariables|GetDañoActor) (/ (LocalVariables|GetCPActor) 1e+02))))

(fn CalculateDefence
  (params (Daño :type Float%20%28double-precision%29) (Defence :type Float%20%28double-precision%29))
  (bind _output_get (LocalVariables|SetDañoActor (|(Dmg-(Dmg*Def)) Daño (/ Defence 1e+02))))
  (if (== _output_get 0.0)
    (return 1.0)
    (else
      (return (LocalVariables|GetDañoActor)))))