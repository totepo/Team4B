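; Pistol interactable for a story event, where the player reacts in subtitles to finding the gun before the parent interaction can run.
; Look-at toggles custom depth on the mesh and, within pickup range, shows a "???" prompt until the event has played.
; The first interaction runs once, disabling input during timed Korean subtitles from the game mode's widget, then increments Count so the next interaction calls the parent's OnInteract.
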(event `/Game/FirstPerson/Blueprints/Interface/BPI_Interactable.OnLookingAt`
  (params (DistanceToPlayer :type "Float (double-precision)") (instigator :type "Actor Object Reference"))
  (bind _bpc_lookat (`/Game/FirstPerson/Blueprints/BP_FirstPersonCharacter.BPC_LookAt` (`self.As BP First Person Character`)))
  (`parent.OnLookingAt` DistanceToPlayer instigator)
  (`PrimitiveComponent.SetRenderCustomDepth` (`self.Test`) true)
  (if (< (`self.Distance to Player`) (`self.pickup Range`))
    (if (> (`self.Count`) 0)
      (`/Game/FirstPerson/Blueprints/Components/BPC_LookAt.getTextToObject` _bpc_lookat (`self.Text`))
      (else
        (`/Game/FirstPerson/Blueprints/Components/BPC_LookAt.getTextToObject` _bpc_lookat "???")))
    (else
      (`/Game/FirstPerson/Blueprints/Components/BPC_LookAt.closeTextToObject` _bpc_lookat))))

(event `/Game/FirstPerson/Blueprints/Interface/BPI_Interactable.OnStoppedLookingAt`
  (params (instigator :type "Actor Object Reference"))
  (`parent.OnStoppedLookingAt` instigator)
  (`PrimitiveComponent.SetRenderCustomDepth` (`self.Test`) false))

(event `/Game/FirstPerson/Blueprints/Interface/BPI_Interactable.OnInteract`
  (params (Instigator :type "Actor Object Reference"))
  (bind _wbp_subtitle (`self.WBP Subtitle`))
  (bind _asbp_first_person_game_mode (cast `/Game/FirstPerson/FrameWork/BP_FirstPersonGameMode` (`GameplayStatics.GetGameMode`)))
  (set `self.WBP Subtitle` (`/Game/FirstPerson/FrameWork/BP_FirstPersonGameMode.WBP_Subtitle` _asbp_first_person_game_mode))
  (switch `int` (`self.Count`)
    (:`0`
      (`/Engine/EditorBlueprintResources/StandardMacros.DoOnce` false
        (:`Completed`
          (`self.DisableInput` (`self.As BP First Person Character`) (`GameplayStatics.GetPlayerController` 0))
          (`/Game/_Proto_Level/Subtitle/WBP_Subtitle.show Subtitle` _wbp_subtitle "권총?!" 1.5)
          (`KismetSystemLibrary.Delay` 2.0)
          (`/Game/_Proto_Level/Subtitle/WBP_Subtitle.show Subtitle` _wbp_subtitle "어째서 여기에 권총이?" 1.5)
          (`KismetSystemLibrary.Delay` 2.0)
          (`/Game/_Proto_Level/Subtitle/WBP_Subtitle.show Subtitle` _wbp_subtitle "일...단 여기 두면 안되니 챙겨두자..." 2.0)
          (`KismetSystemLibrary.Delay` 3.0)
          (`/Engine/EditorBlueprintResources/StandardMacros.IncrementInt` (`self.Count`)
            (:`  `
              (`self.EnableInput` (`self.As BP First Person Character`) (`GameplayStatics.GetPlayerController` 0)))))))
    (:`1`
      (`parent.OnInteract` Instigator))))

(fn `UserConstructionScript`)