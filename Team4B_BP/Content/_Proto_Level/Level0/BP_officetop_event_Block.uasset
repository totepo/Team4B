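; BP_officetop_event_Block is a level event trigger that gates passage with a blocking box until the clock is found.
; On overlap it caches the first-person character and the game mode's subtitle widget, then destroys the block if HaveClock is true.
; Otherwise it activates the block and shows a Korean "clock not found yet" subtitle, which clears when the character leaves.
; The HaveClock check runs for any overlapping actor, outside the character cast.
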(event `self.Box.OnComponentBeginOverlap`
  (params (OverlappedComponent :type "PrimitiveComponent Object Reference") (OtherActor :type "Actor Object Reference") (OtherComp :type "PrimitiveComponent Object Reference") (OtherBodyIndex :type Integer) (bFromSweep :type Boolean) (SweepResult :type "HitResult Structure (by ref)"))
  (bind _text_subtitle (`self.Text Subtitle`))
  (`|ExecutionSequence`
    (:`then_0`
      (bind _asbp_first_person_character (cast `/Game/FirstPerson/Blueprints/BP_FirstPersonCharacter` OtherActor))
      (`/Engine/EditorBlueprintResources/StandardMacros.IsValid` _asbp_first_person_character
        (:`Is Valid`
          (set `self.As BP First Person Character` _asbp_first_person_character)
          (bind _asbp_first_person_game_mode (cast `/Game/FirstPerson/FrameWork/BP_FirstPersonGameMode` (`GameplayStatics.GetGameMode`)))
          (`/Engine/EditorBlueprintResources/StandardMacros.IsValid` _asbp_first_person_game_mode
            (:`Is Valid`
              (bind _wbp_subtitle (`/Game/FirstPerson/FrameWork/BP_FirstPersonGameMode.WBP_Subtitle` _asbp_first_person_game_mode))
              (set `self.WBP Subtitle` _wbp_subtitle)
              (set `self.Text Subtitle` (`/Game/_Proto_Level/Subtitle/WBP_Subtitle.Text_Subtitle` _wbp_subtitle)))))))
    (:`then_1`
      (if (`self.haveClock?`)
        (`ActorComponent.K2_DestroyComponent` (`self.Box_block`))
        (else
          (`ActorComponent.SetActive` (`self.Box_block`) true false)
          (`TextBlock.SetText` _text_subtitle "아직 시계를 찾지 못했어.")
          (`Widget.SetVisibility` _text_subtitle "Visible"))))))

(event `self.Box.OnComponentEndOverlap`
  (params (OverlappedComponent :type "PrimitiveComponent Object Reference") (OtherActor :type "Actor Object Reference") (OtherComp :type "PrimitiveComponent Object Reference") (OtherBodyIndex :type Integer))
  (bind _text_subtitle (`self.Text Subtitle`))
  (bind _asbp_first_person_character (cast `/Game/FirstPerson/Blueprints/BP_FirstPersonCharacter` OtherActor))
  (`/Engine/EditorBlueprintResources/StandardMacros.IsValid` _asbp_first_person_character
    (:`Is Valid`
      (`TextBlock.SetText` _text_subtitle "")
      (`Widget.SetVisibility` _text_subtitle "Hidden"))))

(fn `UserConstructionScript`)