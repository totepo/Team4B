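; Interactable clock prop for the office-top event in the Level0 prototype, built on a parent look-at/interact class.
; While looked at, it enables custom depth on its mesh for highlighting and, within interact range, shows its text through the player character's look-at component, closing it when farther away.
; Looking away clears the highlight, and interaction only forwards to the parent implementation.
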(event `/Game/FirstPerson/Blueprints/Interface/BPI_Interactable.OnLookingAt`
  (params (DistanceToPlayer :type "Float (double-precision)") (instigator :type "Actor Object Reference"))
  (bind _bpc_lookat (`/Game/FirstPerson/Blueprints/BP_FirstPersonCharacter.BPC_LookAt` (`self.As BP First Person Character`)))
  (`parent.OnLookingAt` DistanceToPlayer instigator)
  (`PrimitiveComponent.SetRenderCustomDepth` (`self.StaticMesh`) true)
  (if (< (`self.Distance to Player`) (`self.InteractRange`))
    (`/Game/FirstPerson/Blueprints/Components/BPC_LookAt.getTextToObject` _bpc_lookat (`self.Text`))
    (else
      (`/Game/FirstPerson/Blueprints/Components/BPC_LookAt.closeTextToObject` _bpc_lookat))))

(event `/Game/FirstPerson/Blueprints/Interface/BPI_Interactable.OnStoppedLookingAt`
  (params (instigator :type "Actor Object Reference"))
  (`parent.OnStoppedLookingAt` instigator)
  (`PrimitiveComponent.SetRenderCustomDepth` (`self.StaticMesh`) false))

(event `/Game/FirstPerson/Blueprints/Interface/BPI_Interactable.OnInteract`
  (params (Instigator :type "Actor Object Reference"))
  (`parent.OnInteract` Instigator))

(fn `UserConstructionScript`)