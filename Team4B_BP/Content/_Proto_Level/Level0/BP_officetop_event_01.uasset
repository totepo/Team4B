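; One-shot rooftop story trigger in Level0 that plays the player's Korean monologue about a lost watch, setting up a search before heading down.
; When BP_FirstPersonCharacter first overlaps the Box, it disables input and shows the subtitle widget held by BP_FirstPersonGameMode.
; Hardcoded lines advance through chained Delays; input returns as the last line appears, then the subtitle hides.
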(event `self.Box.OnComponentBeginOverlap`
  (params (OverlappedComponent :type "PrimitiveComponent Object Reference") (OtherActor :type "Actor Object Reference") (OtherComp :type "PrimitiveComponent Object Reference") (OtherBodyIndex :type Integer) (bFromSweep :type Boolean) (SweepResult :type "HitResult Structure (by ref)"))
  (bind _asbp_first_person_character (cast `/Game/FirstPerson/Blueprints/BP_FirstPersonCharacter` OtherActor))
  (`/Engine/EditorBlueprintResources/StandardMacros.IsValid` _asbp_first_person_character
    (:`Is Valid`
      (set `self.As BP First Person Character` _asbp_first_person_character)
      (`/Engine/EditorBlueprintResources/StandardMacros.DoOnce` false
        (:`Completed`
          (bind _asbp_first_person_game_mode (cast `/Game/FirstPerson/FrameWork/BP_FirstPersonGameMode` (`GameplayStatics.GetGameMode`)))
          (`/Engine/EditorBlueprintResources/StandardMacros.IsValid` _asbp_first_person_game_mode
            (:`Is Valid`
              (bind _wbp_subtitle (`/Game/FirstPerson/FrameWork/BP_FirstPersonGameMode.WBP_Subtitle` _asbp_first_person_game_mode))
              (set `self.WBP Subtitle` _wbp_subtitle)
              (set `self.Text Subtitle` (`/Game/_Proto_Level/Subtitle/WBP_Subtitle.Text_Subtitle` _wbp_subtitle))
              (`|ExecutionSequence`
                (:`then_0`
                  (`self.DisableInput` (`self.As BP First Person Character`) null)
                  (`Widget.SetVisibility` (`self.Text Subtitle`) "Visible")
                  (`TextBlock.SetText` (`self.Text Subtitle`) ""))
                (:`then_1`
                  (`TextBlock.SetText` (`self.Text Subtitle`) "잠깐.")
                  (`KismetSystemLibrary.Delay` 2.0)
                  (`TextBlock.SetText` (`self.Text Subtitle`) "내 시계가 어디로 갔지?")
                  (`KismetSystemLibrary.Delay` 2.0)
                  (`TextBlock.SetText` (`self.Text Subtitle`) "")
                  (`KismetSystemLibrary.Delay` 1.0)
                  (`TextBlock.SetText` (`self.Text Subtitle`) "옥상 어디에서 잃어버린 거 같은데...")
                  (`KismetSystemLibrary.Delay` 3.0)
                  (`TextBlock.SetText` (`self.Text Subtitle`) "")
                  (`KismetSystemLibrary.Delay` 1.0)
                  (`TextBlock.SetText` (`self.Text Subtitle`) "얼른 찾고나서 내려가자.")
                  (`self.EnableInput` (`self.As BP First Person Character`) null)
                  (`KismetSystemLibrary.Delay` 3.0)
                  (`Widget.SetVisibility` (`self.Text Subtitle`) "Hidden")
                  (`TextBlock.SetText` (`self.Text Subtitle`) ""))))))))))

(fn `UserConstructionScript`)