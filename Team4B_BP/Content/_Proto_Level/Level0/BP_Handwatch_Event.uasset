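; BP_Handwatch_Event is an interactable wristwatch prop for the Level0 prototype.
; Looking at it enables a custom-depth highlight and shows look-at text within close range, while looking away clears the highlight.
; Interaction only calls the parent, as the map-trigger and self-destroy chains are disconnected.
; Subtitle_send briefly shows a Korean "found the watch, let's head down" line through the GameMode's subtitle widget.
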(event `self.ReceiveBeginPlay`)

(event `/Game/FirstPerson/Blueprints/Interface/BPI_Interactable.OnInteract`
  (params (Instigator :type "Actor Object Reference"))
  (`parent.OnInteract` Instigator))

(event `Subtitle_send`
  (bind _text_subtitle (`self.Text Subtitle`))
  (bind _text_subtitle_2 (`self.Text Subtitle`))
  (bind _asbp_first_person_game_mode (cast `/Game/FirstPerson/FrameWork/BP_FirstPersonGameMode` (`GameplayStatics.GetGameMode`)))
  (`/Engine/EditorBlueprintResources/StandardMacros.IsValid` _asbp_first_person_game_mode
    (:`Is Valid`
      (bind _wbp_subtitle (`/Game/FirstPerson/FrameWork/BP_FirstPersonGameMode.WBP_Subtitle` _asbp_first_person_game_mode))
      (set `self.WBP Subtitle` _wbp_subtitle)
      (set `self.Text Subtitle` (`/Game/_Proto_Level/Subtitle/WBP_Subtitle.Text_Subtitle` _wbp_subtitle))
      (`TextBlock.SetText` _text_subtitle "시계도 찾았으니 이제 내려가보자.")
      (`Widget.SetVisibility` _text_subtitle "Visible")
      (`KismetSystemLibrary.Delay` 3.5)
      (`TextBlock.SetText` _text_subtitle_2 "")
      (`Widget.SetVisibility` _text_subtitle_2 "Hidden"))))

(event `/Game/FirstPerson/Blueprints/Interface/BPI_Interactable.OnLookingAt`
  (params (DistanceToPlayer :type "Float (double-precision)") (instigator :type "Actor Object Reference"))
  (bind _bpc_lookat (`/Game/FirstPerson/Blueprints/BP_FirstPersonCharacter.BPC_LookAt` (`self.As BP First Person Character`)))
  (`parent.OnLookingAt` DistanceToPlayer instigator)
  (`PrimitiveComponent.SetRenderCustomDepth` (`self.StaticMesh`) true)
  (if (< (`self.Distance to Player`) 250.0)
    (`/Game/FirstPerson/Blueprints/Components/BPC_LookAt.getTextToObject` _bpc_lookat (`self.Text`))
    (else
      (`/Game/FirstPerson/Blueprints/Components/BPC_LookAt.closeTextToObject` _bpc_lookat))))

(event `/Game/FirstPerson/Blueprints/Interface/BPI_Interactable.OnStoppedLookingAt`
  (params (instigator :type "Actor Object Reference"))
  (`parent.OnStoppedLookingAt` instigator)
  (`PrimitiveComponent.SetRenderCustomDepth` (`self.StaticMesh`) false))

(fn `UserConstructionScript`)