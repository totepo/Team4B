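; Flashlight pickup actor that grants the first-person character a flashlight, built on a parent with look-at and interact events.
; While looked at, it enables custom depth on its mesh and shows its text through the player's look-at component within close range, closing it beyond.
; Interacting when the player lacks a flashlight sets the ownership flag, toggles the character's flashlight visibility and destroys the pickup.
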(event `/Game/FirstPerson/Blueprints/Interface/BPI_Interactable.OnLookingAt`
  (params (DistanceToPlayer :type "Float (double-precision)") (instigator :type "Actor Object Reference"))
  (bind _bpc_lookat (`/Game/FirstPerson/Blueprints/BP_FirstPersonCharacter.BPC_LookAt` (`self.As BP First Person Character`)))
  (`parent.OnLookingAt` DistanceToPlayer instigator)
  (`PrimitiveComponent.SetRenderCustomDepth` (`self.StaticMesh`) true)
  (if (< (`self.Distance to Player`) 250.0)
    (`/Game/FirstPerson/Blueprints/Components/BPC_LookAt.getTextToObject` _bpc_lookat (`self.Text`))
    (else
      (`/Game/FirstPerson/Blueprints/Components/BPC_LookAt.closeTextToObject` _bpc_lookat))))

(event `/Game/FirstPerson/Blueprints/Interface/BPI_Interactable.OnStoppedLookingAt`
  (params (instigator :type "Actor Object Reference"))
  (`parent.OnStoppedLookingAt` instigator)
  (`PrimitiveComponent.SetRenderCustomDepth` (`self.StaticMesh`) false))

(event `/Game/FirstPerson/Blueprints/Interface/BPI_Interactable.OnInteract`
  (params (Instigator :type "Actor Object Reference"))
  (bind _as_bp_first_person_character (`self.As BP First Person Character`))
  (`parent.OnInteract` Instigator)
  (if (not (`/Game/FirstPerson/Blueprints/BP_FirstPersonCharacter.hasFlashLight` _as_bp_first_person_character))
    (set `/Game/FirstPerson/Blueprints/BP_FirstPersonCharacter.hasFlashLight` true _as_bp_first_person_character)
    (bind _output_get (set `/Game/FirstPerson/Blueprints/BP_FirstPersonCharacter.FlashLightVisiblilty` (not (`/Game/FirstPerson/Blueprints/BP_FirstPersonCharacter.FlashLightVisiblilty` _as_bp_first_person_character)) _as_bp_first_person_character))
    (`SceneComponent.SetVisibility` (`/Game/FirstPerson/Blueprints/BP_FirstPersonCharacter.FlashLight` _as_bp_first_person_character) _output_get false)
    (`self.K2_DestroyActor`)))

(fn `UserConstructionScript`
  (`parent.UserConstructionScript`))