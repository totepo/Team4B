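; Prototype door Blueprint that only activates when the player has a flashlight.
; On interact, it checks that the player is within InteractRange, then calls Activate if the first-person character's HasFlashLight flag is set.
; Otherwise it shows a timed Korean subtitle through the game mode's subtitle widget, saying something seems caught and hinting to find a flashlight to inspect it.
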(event `/Game/FirstPerson/Blueprints/Interface/BPI_Interactable.OnInteract`
  (params (Instigator :type "Actor Object Reference"))
  (if (> (`self.Interact Range`) (`self.Distance to Player`))
    (if (`/Game/FirstPerson/Blueprints/BP_FirstPersonCharacter.hasFlashLight` (`self.As BP First Person Character`))
      (`self.Activate`)
      (else
        (bind _asbp_first_person_game_mode (cast `/Game/FirstPerson/FrameWork/BP_FirstPersonGameMode` (`GameplayStatics.GetGameMode`)))
        (`/Engine/EditorBlueprintResources/StandardMacros.IsValid` _asbp_first_person_game_mode
          (:`Is Valid`
            (`/Game/_Proto_Level/Subtitle/WBP_Subtitle.show Subtitle` (`/Game/FirstPerson/FrameWork/BP_FirstPersonGameMode.WBP_Subtitle` _asbp_first_person_game_mode) "뭔가 걸린거 같은데 어두워서 잘 안보여. \n손전등을 찾아서 살펴보자." 2.0)))))))

(fn `UserConstructionScript`
  (`parent.UserConstructionScript`))