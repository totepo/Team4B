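; BP_Door_Basic4_Locked is a prototype door Blueprint that can refuse interaction while locked.
; On interact, it checks that the player is within interact range, then reads its IsLocked flag.
; A locked door shows a brief hardcoded Korean "It's locked..." subtitle through the subtitle widget held by BP_FirstPersonGameMode; an unlocked one calls Activate.
; The interaction also requires that game mode cast to succeed, even when unlocked.
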(event `/Game/FirstPerson/Blueprints/Interface/BPI_Interactable.OnInteract`
  (params (Instigator :type "Actor Object Reference"))
  (if (> (`self.Interact Range`) (`self.Distance to Player`))
    (bind _asbp_first_person_game_mode (cast `/Game/FirstPerson/FrameWork/BP_FirstPersonGameMode` (`GameplayStatics.GetGameMode`)))
    (`/Engine/EditorBlueprintResources/StandardMacros.IsValid` _asbp_first_person_game_mode
      (:`Is Valid`
        (if (`self.IsLocked`)
          (`/Game/_Proto_Level/Subtitle/WBP_Subtitle.show Subtitle` (`/Game/FirstPerson/FrameWork/BP_FirstPersonGameMode.WBP_Subtitle` _asbp_first_person_game_mode) "잠겨있어..." 2.0)
          (else
            (`self.Activate`)))))))

(fn `UserConstructionScript`
  (`parent.UserConstructionScript`))