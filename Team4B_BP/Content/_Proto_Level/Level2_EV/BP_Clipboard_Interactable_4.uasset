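; Interactable clipboard in the Level 2 prototype that reveals a story document, an employee evaluation listing staff passed over for promotion in 2023.
; Looking at it turns on custom depth highlighting and, at close range, shows prompt text through the player's look-at component; looking away clears the highlight.
; Interacting caches the player character, plays a page-turn sound and shows the Korean document text as a timed subtitle through the game mode's subtitle widget.
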(event `/Game/FirstPerson/Blueprints/Interface/BPI_Interactable.OnLookingAt`
  (params (DistanceToPlayer :type "Float (double-precision)") (instigator :type "Actor Object Reference"))
  (bind _bpc_lookat (`/Game/FirstPerson/Blueprints/BP_FirstPersonCharacter.BPC_LookAt` (`self.As BP First Person Character`)))
  (`parent.OnLookingAt` DistanceToPlayer instigator)
  (`PrimitiveComponent.SetRenderCustomDepth` (`self.Clipboard`) true)
  (if (< (`self.Distance to Player`) 250.0)
    (`/Game/FirstPerson/Blueprints/Components/BPC_LookAt.getTextToObject` _bpc_lookat (`self.Text`))
    (else
      (`/Game/FirstPerson/Blueprints/Components/BPC_LookAt.closeTextToObject` _bpc_lookat))))

(event `/Game/FirstPerson/Blueprints/Interface/BPI_Interactable.OnStoppedLookingAt`
  (params (instigator :type "Actor Object Reference"))
  (`parent.OnStoppedLookingAt` instigator)
  (`PrimitiveComponent.SetRenderCustomDepth` (`self.Clipboard`) false))

(event `/Game/FirstPerson/Blueprints/Interface/BPI_Interactable.OnInteract`
  (params (Instigator :type "Actor Object Reference"))
  (`parent.OnInteract` Instigator)
  (bind _asbp_first_person_character (cast `/Game/FirstPerson/Blueprints/BP_FirstPersonCharacter` Instigator))
  (`/Engine/EditorBlueprintResources/StandardMacros.IsValid` _asbp_first_person_character
    (:`Is Valid`
      (set `self.As BP First Person Character` _asbp_first_person_character)
      (bind _asbp_first_person_game_mode (cast `/Game/FirstPerson/FrameWork/BP_FirstPersonGameMode` (`GameplayStatics.GetGameMode`)))
      (set `self.WBP Subtitle` (`/Game/FirstPerson/FrameWork/BP_FirstPersonGameMode.WBP_Subtitle` _asbp_first_person_game_mode))
      (`GameplayStatics.PlaySound2D` "/Game/_Proto_Level/Level2_EV/페이지_넘기는_소리_.페이지_넘기는_소리_" 1.0 1.0 0.0 null null)
      (`/Game/_Proto_Level/Subtitle/WBP_Subtitle.show Subtitle` (`self.WBP Subtitle`) "직원 평가서2 \n \n[‘23년도 진급누락자 명단’] \n[☐☐☐....XXX…...김창수……" 5.0)
      (`KismetSystemLibrary.Delay` 5.0))))

(fn `UserConstructionScript`)