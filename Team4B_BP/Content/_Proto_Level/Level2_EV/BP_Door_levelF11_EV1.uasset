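; Prototype level door, named for floor 11 of Level2_EV, that the player can activate by interacting with it.
; OnInteract calls Activate only when DistanceToPlayer is less than InteractRange.
; The construction script only calls its parent, and the BeginPlay, overlap and Tick events are disabled stubs.
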(event `/Game/FirstPerson/Blueprints/Interface/BPI_Interactable.OnInteract`
  (params (Instigator :type "Actor Object Reference"))
  (if (> (`self.Interact Range`) (`self.Distance to Player`))
    (`self.Activate`)))

(fn `UserConstructionScript`
  (`parent.UserConstructionScript`))