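; BP_Arm_Boss is an enemy character, by name a boss arm, that handles its death and loot drop.
; Tick watches current HP on CAIEnemyComponet and, once it runs out, disables capsule and mesh collision through a DoOnce.
; When destroyed, it randomly spawns AR or DMR ammo or a health pack, though one branch has no class set.
; Health widget setup and hiding nodes are present but disconnected.
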(event `self.ReceiveBeginPlay`)

(event `self.ReceiveTick`
  (params (DeltaSeconds :type "Float (single-precision)"))
  (bind (_e_statenemy_rangeattack _e_statenemy_maxhp _e_statenemy_currenthp) (break `/Game/AIEnemy_/ComponentEnum-Es/ES_StatEnemy` (`/Game/AIEnemy_/C_AIEnemyComponet.E_StatEnemy` (`self.C_AIEnemyComponet`))))
  (if (not (> _e_statenemy_currenthp 0.0))
    (`/Engine/EditorBlueprintResources/StandardMacros.DoOnce` false
      (:`Completed`
        (`PrimitiveComponent.SetCollisionEnabled` (`self.CapsuleComponent`) "NoCollision")
        (`PrimitiveComponent.SetCollisionEnabled` (`self.Mesh`) "NoCollision")))))

(event `self.ReceiveDestroyed`
  (bind _returnvalue (`self.GetTransform`))
  (switch `int` (`KismetMathLibrary.RandomInteger` 6)
    (:`0`
      (`|SpawnActorFromClass` "/Game/FirstPerson/Blueprints/Weapon/Ammo/BP_item_Ammunition_ar.BP_item_Ammunition_ar_C" _returnvalue "Undefined" "MultiplyWithRoot" null null))
    (:`1`
      (`|SpawnActorFromClass` "/Game/FirstPerson/Blueprints/Weapon/Ammo/BP_item_Ammunition_dmr.BP_item_Ammunition_dmr_C" _returnvalue "Undefined" "MultiplyWithRoot" null null))
    (:`2`
      (`|SpawnActorFromClass` "/Game/FirstPerson/Blueprints/Weapon/Ammo/BP_item_HealthPack.BP_item_HealthPack_C" _returnvalue "Undefined" "MultiplyWithRoot" null null))
    (:`3`
      (`|SpawnActorFromClass` "/Game/FirstPerson/Blueprints/Weapon/Ammo/BP_item_HealthPack.BP_item_HealthPack_C" _returnvalue "Undefined" "MultiplyWithRoot" null null))
    (:`4`
      (`|SpawnActorFromClass` "/Game/FirstPerson/Blueprints/Weapon/Ammo/BP_item_Ammunition_dmr.BP_item_Ammunition_dmr_C" _returnvalue "Undefined" "MultiplyWithRoot" null null))
    (:`5`
      (`|SpawnActorFromClass` "/Game/FirstPerson/Blueprints/Weapon/Ammo/BP_item_Ammunition_ar.BP_item_Ammunition_ar_C" _returnvalue "Undefined" "MultiplyWithRoot" null null))))

(fn `UserConstructionScript`)