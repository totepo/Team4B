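; Monster eye enemy Blueprint with a health widget, apparently an unused variant going by its asset name.
; BeginPlay creates the health widget, assigns it to the UIHP component and passes it the enemy AI component that holds the stats.
; Tick polls current HP; once it is no longer above zero, a DoOnce disables capsule and mesh collision and hides the health widget.
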(event `self.ReceiveBeginPlay`
  (bind _returnvalue (`|CreateWidget` "/Game/AIEnemy_/Widget/WidgetSalud.WidgetSalud_C" null null))
  (`WidgetComponent.SetWidget` (`self.UIHP`) _returnvalue)
  (set `/Game/AIEnemy_/Widget/WidgetSalud.AIComponet` (`self.C_AIEnemyComponet`) _returnvalue))

(event `self.ReceiveTick`
  (params (DeltaSeconds :type "Float (single-precision)"))
  (bind (_e_statenemy_rangeattack _e_statenemy_maxhp _e_statenemy_currenthp) (break `/Game/AIEnemy_/ComponentEnum-Es/ES_StatEnemy` (`/Game/AIEnemy_/C_AIEnemyComponet.E_StatEnemy` (`self.C_AIEnemyComponet`))))
  (if (not (> _e_statenemy_currenthp 0.0))
    (`/Engine/EditorBlueprintResources/StandardMacros.DoOnce` false
      (:`Completed`
        (`PrimitiveComponent.SetCollisionEnabled` (`self.CapsuleComponent`) "NoCollision")
        (`PrimitiveComponent.SetCollisionEnabled` (`self.Mesh`) "NoCollision")
        (`SceneComponent.SetVisibility` (`self.UIHP`) false false)))))

(fn `UserConstructionScript`)