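; BP_Door_Basic1 is a hinged level door that swings open and closed when its Activate event fires, unless IsLocked or HingeMode is set.
; HingeLeftRight selects one of two timelines, and the Open flag flips on each activation to play or reverse it.
; The timeline's DoorOpening value plus RelativeYaw drives the Door component's relative yaw, leaving roll and pitch unchanged.
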(event `self.ReceiveBeginPlay`
  (`parent.ReceiveBeginPlay`))

(event `/Game/BrutalistLevelKit/Blueprints/Furniture/Parent/BI_LevelObjectInteraction.Activate`
  (bind _door (`self.Door`))
  (bind _door_2 (`self.Door`))
  (bind (_relativerotation_roll _relativerotation_pitch) (`KismetMathLibrary.BreakRotator` (`SceneComponent.RelativeRotation` _door_2)))
  (bind (_relativerotation_roll_2 _relativerotation_pitch_2) (`KismetMathLibrary.BreakRotator` (`SceneComponent.RelativeRotation` _door)))
  (if (or (`self.IsLocked`) (`self.HingeMode`))
    _
    (elif (`self.HingeLeftRight`)
      (if (`self.Open`)
        ;[1 1 1] Level Object Activation
        (set `self.Open` false)
        (bind (_direction _dooropening) (`Timeline|Timeline_0` :!label _label)
          (:`Update`
            (`SceneComponent.K2_SetRelativeRotation` _door_2 (`KismetMathLibrary.MakeRotator` _relativerotation_roll _relativerotation_pitch (+ _dooropening (`self.RelativeYaw`))) false false)))
        (else
          (set `self.Open` true)
          (goto _label :!via `Reverse`)))
      (elif (`self.Open`)
        ;[1 1 1] Level Object Activation
        (set `self.Open` false)
        (bind (_direction_2 _dooropening_2) (`Timeline|Timeline_1` :!label _label_2)
          (:`Update`
            (`SceneComponent.K2_SetRelativeRotation` _door (`KismetMathLibrary.MakeRotator` _relativerotation_roll_2 _relativerotation_pitch_2 (+ _dooropening_2 (`self.RelativeYaw`))) false false)))
        (else
          (set `self.Open` true)
          (goto _label_2 :!via `Reverse`))))))

(fn `UserConstructionScript`
  (`parent.UserConstructionScript`))