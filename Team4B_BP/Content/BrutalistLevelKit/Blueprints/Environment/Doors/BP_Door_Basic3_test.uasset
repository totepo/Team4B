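; A test variant of a basic door Blueprint that swings the Door component open and closed when activated.
; BeginPlay stores the door's starting relative yaw, and a timeline adds its DoorOpening curve to that yaw while preserving roll and pitch.
; Each Activate flips the Open flag and plays or reverses the timeline, but does nothing if the door is locked or in hinge mode.
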(event `self.ReceiveBeginPlay`
  (bind (_relativerotation_roll _relativerotation_pitch _relativerotation_yaw) (`KismetMathLibrary.BreakRotator` (`SceneComponent.RelativeRotation` (`self.Door`))))
  (`parent.ReceiveBeginPlay`)
  (set `self.RelativeYaw_0` _relativerotation_yaw))

(event `/Game/BrutalistLevelKit/Blueprints/Furniture/Parent/BI_LevelObjectInteraction.Activate`
  (bind _door (`self.Door`))
  (bind (_relativerotation_roll _relativerotation_pitch) (`KismetMathLibrary.BreakRotator` (`SceneComponent.RelativeRotation` _door)))
  (if (not (or (`self.IsLocked`) (`self.HingeMode`)))
    ;[1 1 1] Level Object Activation
    (if (`self.Open`)
      (set `self.Open` false)
      (bind (_direction _dooropening) (`Timeline|Timeline_0` :!label _label)
        (:`Update`
          (`SceneComponent.K2_SetRelativeRotation` _door (`KismetMathLibrary.MakeRotator` _relativerotation_roll _relativerotation_pitch (+ _dooropening (`self.RelativeYaw_0`))) false false)))
      (else
        (set `self.Open` true)
        (goto _label :!via `Reverse`)))))

(fn `UserConstructionScript`
  (`parent.UserConstructionScript`))